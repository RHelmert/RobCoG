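; Multiplayer Manus glove body pawn that lets up to four color-coded players grab objects with hand gestures.
; On possession it moves to its tagged Player Start, spawns a CopyCat of itself in front, takes ownership of tagged actors and registers the CopyCat with their switches and dials.
; RepNotifies color the CopyCat by PlayerId.
; Grab gestures drive BPI_Grabbable through per-hand overlap boxes, which also vibrate the glove on touch.
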(event OnGestureStarted(ManusBody)
  (params (HandType :type EManusHandType%20Enum :default "Left") (GestureName :type Name :default "None"))
  ;[1 1 1] Hand gesture started
  (CallFunction|LogGestureDetected HandType GestureName true))

(event OnGestureonGoing(ManusBody)
  (params (HandType :type EManusHandType%20Enum :default "Left") (GestureName :type Name :default "None") (Duration :type Float%20%28single-precision%29))
  ;[1 1 1] Hand gesture on-going - Try to grab
  (if (and (Utilities|IsGrabGesture GestureName) (<= Duration 0.25))
    (CallFunction|TryGrabbing HandType)))

(event OnGestureFinished(ManusBody)
  (params (HandType :type EManusHandType%20Enum :default "Left") (GestureName :type Name :default "None"))
  ;[1 1 1] Hand gesture finished - Try to ungrab
  (CallFunction|LogGestureDetected HandType GestureName false)
  (if (Utilities|IsGrabGesture GestureName)
    (CallFunction|TryUngrabbing HandType)))

(event OnComponentBeginOverlap(GrabBoxLeft)
  (params (OverlappedComponent :type Primitive%20Component%20Object%20Reference) (OtherActor :type Actor%20Object%20Reference) (OtherComp :type Primitive%20Component%20Object%20Reference) (OtherBodyIndex :type Integer) (bFromSweep :type Boolean) (SweepResult :type Hit%20Result%20Structure%20%28by%20ref%29))
  ;[1 1 1] Hand vibration when touching a grabbable
  (Utilities|Casting|CastToBPI_Grabbable OtherActor)
  (Class|ManusComponent|VibrateManusGloveHand (Variables|Default|GetManusBody) "Left" 0.6 300))

(event OnComponentBeginOverlap(GrabBoxRight)
  (params (OverlappedComponent :type Primitive%20Component%20Object%20Reference) (OtherActor :type Actor%20Object%20Reference) (OtherComp :type Primitive%20Component%20Object%20Reference) (OtherBodyIndex :type Integer) (bFromSweep :type Boolean) (SweepResult :type Hit%20Result%20Structure%20%28by%20ref%29))
  ;[1 1 1] Hand vibration when touching a grabbable
  (Utilities|Casting|CastToBPI_Grabbable OtherActor)
  (Class|ManusComponent|VibrateManusGloveHand (Variables|Default|GetManusBody) "Right" 0.6 300))

(event EventPossessed
  (params (NewController :type Controller%20Object%20Reference))
  (bind _returnvalue (Transformation|GetActorTransform))
  (bind _playerstate (Variables|/Script/Engine.Controller|GetPlayerState NewController))
  ;[1 1 1] Possessed: Place each player at a Player Start based on their Player ID, assign him a color, set the owner of the actors of that color, create copy cat
  (Utilities|IsValid _playerstate
    (:Is%20Valid
      (bind _outactors (Actor|GetAllActorsOfClasswithTag "/Script/Engine.PlayerStart" (Utilities|String|StringToName (Utilities|String|Append "PlayerStart" (Utilities|String|ToString(Integer) (+ (Math|Integer|%(Integer) (Variables|/Script/Engine.PlayerState|GetPlayerId _playerstate) 4) 1))))))
      (Utilities|IsValid (Utilities|Array|Get(acopy) _outactors)
        (:Is%20Valid
          (Transformation|SetActorTransform (Transformation|GetActorTransform (Utilities|Array|Get(acopy) _outactors)) false true)
          (bind _returnvalue_2 (Game|SpawnActorfromClass (Utilities|GetClass self) (Math|Transform|MakeTransform (+ (* (Transformation|GetActorForwardVector) 200) (.location _returnvalue)) (Math|Rotator|CombineRotators (.rotation _returnvalue) "0,180.000000, 0") (.scale _returnvalue)) "AlwaysSpawn" self 0))
          (Variables|Default|SetCopyCat _returnvalue_2)
          (Variables|Default|SetPlayerId (Math|Integer|%(Integer) (Variables|/Script/Engine.PlayerState|GetPlayerId _playerstate) 4))
          (bind _outactors_2 (Actor|GetAllActorsOfClasswithTag "/Script/Engine.Actor" (Utilities|String|StringToName (Utilities|String|Append "Player" (Utilities|String|ToString(Integer) (+ (Math|Integer|%(Integer) (Variables|/Script/Engine.PlayerState|GetPlayerId _playerstate) 4) 1)) "Actor"))))
          (for _array_element _outactors_2
            (Utilities|IsValid _array_element
              (:Is%20Valid
                (Actor|SetOwner _array_element (Pawn|GetController))
                (bind _asbp_rocker_switch_visibility (Utilities|Casting|CastToBP_RockerSwitch_Visibility _array_element)
                  (:then
                    (Default|AddActor _asbp_rocker_switch_visibility (Variables|Default|GetCopyCat)))
                  (:CastFailed
                    (bind _asbp_dial_knob_rotator (Utilities|Casting|CastToBP_DialKnob_Rotator _array_element))
                    (Default|AddActor _asbp_dial_knob_rotator (Variables|Default|GetCopyCat))))))))))))

(event EventOnGrabbedActorGrabbedbySomethingElse
  (params (GrabbedActor :type Actor%20Object%20Reference))
  ;[1 1 1] Hand gesture finished - Try to ungrab
  (if (== GrabbedActor (Variables|Default|GetGrabbedActorLeft))
    (CallFunction|TryUngrabbing "Left")
    (elif (== GrabbedActor (Variables|Default|GetGrabbedActorRight))
      (CallFunction|TryUngrabbing "Right"))))

(event EventEndPlay
  (params (EndPlayReason :type EEndPlayReason%20Enum :default "Destroyed"))
  (bind _copycat (Variables|Default|GetCopyCat))
  ;[1 1 1] End Play
  (Utilities|IsValid _copycat
    (:Is%20Valid
      (Actor|DestroyActor _copycat))))

(fn ConstructionScript)

(fn LogGestureDetected
  (params (HandType :type EManusHandType%20Enum :default "Left") (GestureName :type Name) (StartedVsFinished :type Boolean))
  (Development|PrintString (Utilities|String|Append (Utilities|String|ToString(Name) GestureName) " gesture detection " (select StartedVsFinished "started" "finished") " on the " (Utilities|Select :Index HandType :Left "Left" :Right "Right") " hand.") true true (Math|Color|SelectColor "(R=1.000000,G=0.840063,B=0.000000,A=1.000000)" "(R=1.000000,G=0.360740,B=0.000000,A=1.000000)" StartedVsFinished)))

(fn TryGrabbing
  (params (HandType :type EManusHandType%20Enum :default "Left"))
  (if (not (Utilities|IsGrabbing HandType))
    (bind _output_get (LocalVariables|SetOverlappingGrabbableActors (Collision|GetOverlappingActors (Utilities|Select :Index HandType :Left (Variables|Default|GetGrabBoxLeft) :Right (Variables|Default|GetGrabBoxRight)) "/Script/Engine.Actor" :!class /Script/Engine.PrimitiveComponent)))
    (bind (_arrayindex _arrayelement) (Utilities|Array|ReverseforEachLoop _output_get)
      (:LoopBody
        (Utilities|Casting|CastToBPI_Grabbable _arrayelement
          (:CastFailed
            (Utilities|Array|RemoveIndex (LocalVariables|GetOverlappingGrabbableActors) _arrayindex))))
      (:Completed
        (if (Utilities|Array|IsValidIndex (LocalVariables|GetOverlappingGrabbableActors))
          (bind _asbpi_grabbable (Utilities|Casting|CastToBPI_Grabbable (Utilities|Array|Get(acopy) (LocalVariables|GetOverlappingGrabbableActors))))
          (Default|OnGrabbed _asbpi_grabbable (Pawn|GetController) (Utilities|Select :Index HandType :Left (Variables|Default|GetGrabBoxLeft) :Right (Variables|Default|GetGrabBoxRight)))
          (switch Utilities|FlowControl|Switch|SwitchonEManusHandType HandType
            (:Left
              (Variables|Default|SetGrabbedActorLeft (Utilities|Array|Get(acopy) (LocalVariables|GetOverlappingGrabbableActors))))
            (:Right
              (Variables|Default|SetGrabbedActorRight (Utilities|Array|Get(acopy) (LocalVariables|GetOverlappingGrabbableActors))))))))))

(fn TryUngrabbing
  (params (HandType :type EManusHandType%20Enum :default "Left"))
  (bind _asbpi_grabbable (Utilities|Casting|CastToBPI_Grabbable (Utilities|Select :Index HandType :Left (Variables|Default|GetGrabbedActorLeft) :Right (Variables|Default|GetGrabbedActorRight))))
  (Default|OnUngrabbed _asbpi_grabbable)
  (switch Utilities|FlowControl|Switch|SwitchonEManusHandType HandType
    (:Left
      (Variables|Default|SetGrabbedActorLeft 0))
    (:Right
      (Variables|Default|SetGrabbedActorRight 0))))

(fn OnRepCopyCat
  (CallFunction|UpdateCopyCatColor))

(fn OnRepPlayerId
  (CallFunction|UpdateCopyCatColor))

(fn UpdateCopyCatColor
  (bind _copycat (Variables|Default|GetCopyCat))
  (Utilities|IsValid _copycat
    (:Is%20Valid
      (Rendering|Material|SetMaterial (Variables|BP_ManusGlovesPawn_Body_C|GetManusBody _copycat) 0 (Utilities|Select :Index (Variables|Default|GetPlayerId) :Option%200 "/Manus/Materials/M_Color_Blue.M_Color_Blue" :Option%201 "/Manus/Materials/M_Color_Red.M_Color_Red" :Option%202 "/Manus/Materials/M_Color_Yellow.M_Color_Yellow" :Option%203 "/Manus/Materials/M_Color_Green.M_Color_Green"))
      (Components|Arrow|SetArrowColor(LinearColor) (Variables|BP_ManusGlovesPawn_Body_C|GetArrow (Variables|Default|GetCopyCat)) (Utilities|Select :Index (Variables|Default|GetPlayerId) :Option%200 "(R=0.000000,G=0.149960,B=0.502886,A=1.000000)" :Option%201 "(R=0.300544,G=0.000000,B=0.000000,A=1.000000)" :Option%202 "(R=0.806952,G=0.502886,B=0.000000,A=1.000000)" :Option%203 "(R=0.000000,G=0.149960,B=0.000000,A=1.000000)")))))