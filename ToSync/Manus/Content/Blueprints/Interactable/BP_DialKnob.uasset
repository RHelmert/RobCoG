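; Grabbable dial knob that turns with the component holding it and keeps an angle value, clamped to Range unless both bounds are equal.
; The local controller's grab enables Tick, which turns frame-to-frame changes in signed grab angle into value changes and rotates CursorRotator.
; Each tick sends value and delta through ServerOnValueChanged to MultiOnValueChanged, which is empty here.
; Releasing the knob disables Tick.
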(event Custom|ServerOnValueChanged
  (params (NewValue :type Float%20%28single-precision%29) (DeltaValue :type Float%20%28single-precision%29))
  ;[1 1 1] Server
  (CallFunction|MultionValueChanged NewValue DeltaValue))

(event Custom|MultiOnValueChanged
  (params (NewValue :type Float%20%28single-precision%29) (DeltaValue :type Float%20%28single-precision%29))
  ;[1 1 1] Server
)

(event EventTick
  (params (DeltaSeconds :type Float%20%28single-precision%29))
  (bind _angle (Utilities|CursorGrabbedAngle))
  (bind _range (Variables|Default|GetRange))
  ;[1 1 1] Interaction on the Clients
  (Variables|Default|SetDelta (- (Variables|Default|GetPreviousCursorGrabbedAngle) _angle))
  (Variables|Default|SetPreviousCursorGrabbedAngle _angle)
  (Variables|Default|SetDeltaValue (- (Math|Float|SelectFloat (- (Variables|Default|GetValue) (Variables|Default|GetDelta)) (Math|Float|ClampAngle (- (Variables|Default|GetValue) (Variables|Default|GetDelta)) (.value (.lowerbound _range)) (.value (.upperbound _range))) (== (.value (.lowerbound _range)) (.value (.upperbound _range)))) (Variables|Default|GetValue)))
  (Variables|Default|SetValue (Math|Float|SelectFloat (- (Variables|Default|GetValue) (Variables|Default|GetDelta)) (Math|Float|ClampAngle (- (Variables|Default|GetValue) (Variables|Default|GetDelta)) (.value (.lowerbound _range)) (.value (.upperbound _range))) (== (.value (.lowerbound _range)) (.value (.upperbound _range)))))
  (Transformation|SetRelativeRotation (Variables|Default|GetCursorRotator) (Math|Rotator|MakeRotator 0.0 0.0 (* (Variables|Default|GetValue) -1.0)) false false)
  (CallFunction|ServeronValueChanged (Variables|Default|GetValue) (Variables|Default|GetDeltaValue)))

(event EventOnUngrabbed
  (params (Instigator :type Controller%20Object%20Reference))
  ;[1 1 1] Interaction on the Clients
  (Actor|Tick|SetActorTickEnabled false)
  (Variables|Default|SetGrabbingActor 0))

(event EventOnGrabbed
  (params (Instigator :type Controller%20Object%20Reference) (AttachComponent :type Scene%20Component%20Object%20Reference))
  ;[1 1 1] Interaction on the Clients
  (Utilities|IsValid Instigator
    (:Is%20Valid
      (if (Pawn|IsLocalController Instigator)
        (Utilities|IsValid (Variables|Default|GetGrabbingActor)
          (:Is%20Valid
            (Class|BPIGrabber|OnGrabbedActorGrabbedbySomethingElse(Message) (Variables|Default|GetGrabbingActor) self))
          (:Is%20Not%20Valid
            _))
        (bind _output_get (Variables|Default|SetGrabbingActor (Components|GetOwner AttachComponent)))
        (Utilities|IsValid _output_get
          (:Is%20Valid
            (Variables|Default|SetGrabbingComponent AttachComponent)
            (Variables|Default|SetPreviousCursorGrabbedAngle (Utilities|CursorGrabbedAngle))
            (Variables|Default|SetCursorRotationAtGrab (Transformation|GetWorldRotation (Variables|Default|GetCursorRotator)))
            (Actor|Tick|SetActorTickEnabled true)))))))

(fn ConstructionScript)