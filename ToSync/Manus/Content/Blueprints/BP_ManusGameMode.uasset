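; Game mode for the Manus demo that shows a setup menu or spawns and possesses a full-body, one-mesh hands or two-mesh hands pawn.
; StartDemo spawns the pawn directly, or for multiplayer menu starts opens a listen server or joins an IP with the choice as a Pawn URL option.
; That option skips the menu on load, and HandleStartingNewPlayer parses it from each join request URL to spawn the requested pawn.
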(event EventBeginPlay
  (bind _optionsstring (Variables|Default|GetOptionsString))
  (bind _returnvalue (Class|GameplayStatics|ParseOption _optionsstring "IP"))
  (bind _returnvalue_2 (Class|GameplayStatics|ParseOption _optionsstring "Pawn"))
  (if (Utilities|Array|IsEmpty _returnvalue_2)
    (Class|HeadMountedDisplayFunctionLibrary|EnableHMD false)
    (bind _returnvalue_3 (UserInterface|CreateWidget "/Manus/UI/UI_ManusDemoMenu.UI_ManusDemoMenu_C"))
    (Utilities|IsValid _returnvalue_3
      (:Is%20Valid
        (UserInterface|Viewport|AddtoViewport _returnvalue_3 0)))
    (else
      (CallFunction|StartDemo (Game|GetPlayerController 0) false true (Utilities|Array|IsEmpty _returnvalue) _returnvalue false (Utilities|Enum|Equal(Enum) _returnvalue_2 "FullBody") (Utilities|Enum|Equal(Enum) _returnvalue_2 "HandsOne")))))

(event EventHandleStartingNewPlayer
  (params (NewPlayer :type Player%20Controller%20Object%20Reference))
  (bind _returnvalue (Class|ManusBlueprintLibrary|GetPlayerJoinRequestURL NewPlayer)) ; Extract client requested Pawn option from client join request URL
  (if (not (Utilities|Array|IsEmpty (Utilities|String|Left (Utilities|String|RightChop _returnvalue (+ (Utilities|String|FindSubstring _returnvalue "?Pawn=" true) 6)) (Utilities|String|FindSubstring (Utilities|String|RightChop _returnvalue (+ (Utilities|String|FindSubstring _returnvalue "?Pawn=" true) 6)) "?"))))
    (CallFunction|StartDemo NewPlayer false true false "" false (Utilities|Enum|Equal(Enum) (Utilities|String|Left (Utilities|String|RightChop _returnvalue (+ (Utilities|String|FindSubstring _returnvalue "?Pawn=" true) 6)) (Utilities|String|FindSubstring (Utilities|String|RightChop _returnvalue (+ (Utilities|String|FindSubstring _returnvalue "?Pawn=" true) 6)) "?")) "FullBody") (Utilities|Enum|Equal(Enum) (Utilities|String|Left (Utilities|String|RightChop _returnvalue (+ (Utilities|String|FindSubstring _returnvalue "?Pawn=" true) 6)) (Utilities|String|FindSubstring (Utilities|String|RightChop _returnvalue (+ (Utilities|String|FindSubstring _returnvalue "?Pawn=" true) 6)) "?")) "HandsOne"))))

(fn ConstructionScript)

(fn StartDemo
  (params (PlayerController :type Player%20Controller%20Object%20Reference) (IsStartedFromMenu :type Boolean) (UseMultiplayer :type Boolean) (UseMultiplayerHost :type Boolean) (IP :type String) (UseVR :type Boolean) (UseFullBodyTracking :type Boolean) (UseOneSkeletalMeshForHandTracking :type Boolean))
  (Utilities|FlowControl|Sequence
    (:then_0
      (if (or (not IsStartedFromMenu) (not UseMultiplayer))
        (bind _returnvalue (Game|SpawnActorfromClass (select UseFullBodyTracking "/Manus/Blueprints/Pawns/BP_ManusPolygonPawn.BP_ManusPolygonPawn_C" (select UseOneSkeletalMeshForHandTracking "/Manus/Blueprints/Pawns/BP_ManusGlovesPawn_Body.BP_ManusGlovesPawn_Body_C" "/Manus/Blueprints/Pawns/BP_ManusGlovesPawn_Hands.BP_ManusGlovesPawn_Hands_C")) (Math|Transform|MakeTransform "0, 0, 0") "AlwaysSpawn" 0 0))
        (bind _aspawn (Utilities|Casting|CastToPawn _returnvalue))
        (Pawn|Possess PlayerController _aspawn)))
    (:then_1
      (if IsStartedFromMenu
        (Class|HeadMountedDisplayFunctionLibrary|EnableHMD UseVR)))
    (:then_2
      (if IsStartedFromMenu
        (if UseMultiplayer
          (Game|OpenLevel(byName) (select UseMultiplayerHost "ManusDemo" (Utilities|String|StringToName IP)) true (Utilities|String|Append "Pawn=" (select UseFullBodyTracking "FullBody" (select UseOneSkeletalMeshForHandTracking "HandsOne" "HandsTwo")) (select UseMultiplayerHost "?listen" ""))))))))