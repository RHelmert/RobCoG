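; ConstraintSetup is a component that configures a physics constraint at BeginPlay for drawer-like sliding or rotating objects.
; It enables owner physics from code, warning if already simulating, because level streaming otherwise breaks constraints.
; Unless the category is DefaultPlain, it uses the assigned or an attached constraint, with optional linear damping.
; It locks all axes, frees the chosen one, and offsets the reference frame by half the range for one-sided travel.
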(event EventTick
  (params (DeltaSeconds :type Float%20%28single-precision%29)))

(event EventBeginPlay
  (bind _returnvalue (Components|GetOwner))
  (bind _drawerextendlength_rotationoffset (Variables|Default|GetDrawerExtendLength/RotationOffset))
  (bind _returnvalue_2 (Actor|GetComponentbyClass _returnvalue "/Script/Engine.PrimitiveComponent"))
  (bind _returnvalue_3 (/ _drawerextendlength_rotationoffset 2.0))
  ;[1 1 1] Check wheter physics is really turned off (it has to be)
  (if (Physics|IsSimulatingPhysics _returnvalue_2 "None")
    ;[1 1 1] Debug: The physics needs to be turned off at start. Otherwise when the constrained is used in level streaming iit would break
    (Development|PrintString (Utilities|String|Append "Physics of the Actor: " (Utilities|GetDisplayName _returnvalue) " should be disabled at start. It will be enabled by code. Else it may cause physics constraints break on level streaming.") true true "(R=1.000000,G=0.789221,B=0.000000,A=1.000000)" 5.0))
  ;[1 1 1] Now enable physics simulation. This has do be done per code, because otherwise the level streaming would break the physics constraints
  (Physics|SetSimulatePhysics _returnvalue_2 true)
  ;[1 1 1] When nothing is chosen just stop here and use the constraints configuration
  (if (Utilities|Enum|NotEqual(Enum) (Variables|Default|GetConstraintCategory) "NewEnumerator9")
    ;[1 1 1] Choose whether to use the given physics constraint or ffind one amongs the children of the component that owns this component
    (if (Utilities|IsValid (Variables|Default|GetPhysicConstraint))
      (Variables|Default|SetUsedConstrainedComp (Variables|/Script/Engine.PhysicsConstraintActor|GetConstraintComp (Variables|Default|GetPhysicConstraint)))
      (else
        ;[1 1 1] Loop through all attached actors
        (for _array_element (Actor|GetAttachedActors _returnvalue true)
          ;[1 1 1] Save the physics constraint that is found
          (if (== (Utilities|GetClass _array_element) "/Script/Engine.PhysicsConstraintActor")
            (bind _asphysics_constraint_actor (Utilities|Casting|CastToPhysicsConstraintActor _array_element))
            (Variables|Default|SetUsedConstrainedComp (Variables|/Script/Engine.PhysicsConstraintActor|GetConstraintComp _asphysics_constraint_actor))))))
    ;[1 1 1] Debug when there is no physics constraint
    (if (Utilities|IsValid (Variables|Default|GetUsedConstrainedComp))
      (if (Variables|Default|GetUseLinearDampening)
        (Class|PhysicsConstraintComponent|SetLinearVelocityDrive (Variables|Default|GetUsedConstrainedComp) true true true)
        (Class|PhysicsConstraintComponent|SetLinearVelocityTarget (Variables|Default|GetUsedConstrainedComp) (Math|Vector|MakeVector 0.0 0.0 0.0))
        (Class|PhysicsConstraintComponent|SetLinearDriveParams (Variables|Default|GetUsedConstrainedComp) 0.0 (Variables|Default|GetDampeningValue) 0.0))
      (Transformation|SetRelativeRotation (Variables|Default|GetUsedConstrainedComp) "0, 0, 0" false true)
      (Class|PhysicsConstraintComponent|SetDisableCollision (Variables|Default|GetUsedConstrainedComp) true)
      (Utilities|FlowControl|Sequence
        (:then_0
          ;[1 1 1] Set all Limits to locked (NOTE: Limit size is always the same reference so setting it not at the end would overwrite the limit in the next step)
          (Class|PhysicsConstraintComponent|SetAngularSwing1Limit (Variables|Default|GetUsedConstrainedComp) "ACM_Locked" 0.0)
          (Class|PhysicsConstraintComponent|SetAngularSwing2Limit (Variables|Default|GetUsedConstrainedComp) "ACM_Locked" 0.0)
          (Class|PhysicsConstraintComponent|SetAngularTwistLimit (Variables|Default|GetUsedConstrainedComp) "ACM_Locked" 0.0))
        (:then_1
          (Class|PhysicsConstraintComponent|SetLinearXLimit (Variables|Default|GetUsedConstrainedComp) "LCM_Locked" 0.0)
          (Class|PhysicsConstraintComponent|SetLinearYLimit (Variables|Default|GetUsedConstrainedComp) "LCM_Locked" 0.0)
          (Class|PhysicsConstraintComponent|SetLinearZLimit (Variables|Default|GetUsedConstrainedComp) "LCM_Locked" 0.0))
        (:then_2
          (switch Utilities|FlowControl|Switch|SwitchonConstraintCategory (Variables|Default|GetConstraintCategory)
            (:NewEnumerator0
              (Class|PhysicsConstraintComponent|SetLinearXLimit (Variables|Default|GetUsedConstrainedComp) "LCM_Limited" _returnvalue_3)
              (Variables|Default|Setx_Offset (* -1 _returnvalue_3)))
            (:NewEnumerator1
              (Class|PhysicsConstraintComponent|SetLinearYLimit (Variables|Default|GetUsedConstrainedComp) "LCM_Limited" _returnvalue_3)
              (Variables|Default|Sety_Offset (* -1 _returnvalue_3)))
            (:NewEnumerator2
              (Class|PhysicsConstraintComponent|SetLinearZLimit (Variables|Default|GetUsedConstrainedComp) "LCM_Limited" _returnvalue_3)
              (Variables|Default|Setz_Offset (* -1 _returnvalue_3)))
            (:NewEnumerator3
              (Class|PhysicsConstraintComponent|SetAngularTwistLimit (Variables|Default|GetUsedConstrainedComp) "ACM_Limited" _returnvalue_3)
              (Variables|Default|SetrotationOffset (Math|Rotator|MakeRotator _returnvalue_3 0.0 0.0)))
            (:NewEnumerator4
              (Class|PhysicsConstraintComponent|SetAngularTwistLimit (Variables|Default|GetUsedConstrainedComp) "ACM_Limited" _returnvalue_3)
              (Variables|Default|SetrotationOffset (Math|Rotator|MakeRotator (* -1 _returnvalue_3) 0.0 0.0)))
            (:NewEnumerator5
              (Class|PhysicsConstraintComponent|SetAngularSwing2Limit (Variables|Default|GetUsedConstrainedComp) "ACM_Limited" _returnvalue_3)
              (Variables|Default|SetrotationOffset (Math|Rotator|MakeRotator 0.0 _returnvalue_3 0.0)))
            (:NewEnumerator6
              (Class|PhysicsConstraintComponent|SetAngularSwing2Limit (Variables|Default|GetUsedConstrainedComp) "ACM_Limited" _returnvalue_3)
              (Variables|Default|SetrotationOffset (Math|Rotator|MakeRotator 0.0 (* -1 _returnvalue_3) 0.0)))
            (:NewEnumerator7
              (Class|PhysicsConstraintComponent|SetAngularSwing1Limit (Variables|Default|GetUsedConstrainedComp) "ACM_Limited" _returnvalue_3)
              (Variables|Default|SetrotationOffset (Math|Rotator|MakeRotator 0.0 0.0 (* -1 _returnvalue_3))))
            (:NewEnumerator8
              (Class|PhysicsConstraintComponent|SetAngularSwing1Limit (Variables|Default|GetUsedConstrainedComp) "ACM_Limited" _returnvalue_3)
              (Variables|Default|SetrotationOffset (Math|Rotator|MakeRotator 0.0 0.0 _returnvalue_3)))))
        (:then_3
          ;[1 1 1] Now add Offset to the respective direction or rotation
          (Class|PhysicsConstraintComponent|SetConstraintReferenceFrame (Variables|Default|GetUsedConstrainedComp) "Frame2" (Math|Transform|MakeTransform (+ (.Location (Math|Transform|BreakTransform (Transformation|GetRelativeTransform (Variables|Default|GetUsedConstrainedComp)))) (Math|Transform|TransformDirection (Transformation|GetRelativeTransform (Variables|Default|GetUsedConstrainedComp)) (Math|Vector|MakeVector (Variables|Default|Getx_Offset) (Variables|Default|Gety_Offset) (Variables|Default|Getz_Offset)))) (Math|Rotator|CombineRotators (.Rotation (Math|Transform|BreakTransform (Transformation|GetRelativeTransform (Variables|Default|GetUsedConstrainedComp)))) (Variables|Default|GetrotationOffset)) (.Scale (Math|Transform|BreakTransform (Transformation|GetRelativeTransform (Variables|Default|GetUsedConstrainedComp))))))))
      (else
        (Development|PrintString "Error: No physics constraint found or set" true true "(R=1.000000,G=0.012011,B=0.000000,A=1.000000)")))))